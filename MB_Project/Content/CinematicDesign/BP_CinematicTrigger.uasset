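; Trigger actor that plays a Level Sequence once when the player character overlaps it.
; On overlap it casts to BP_MB_ProjectCharacter, then creates a sequence player from its LevelSequence and SequenceSettings variables and plays it.
; A HasPlayed flag blocks replays, and debug print strings trace each step.
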(event EventBeginPlay)

(event Collision|EventActorBeginOverlap
  (params (OtherActor :type Actor%20Object%20Reference))
  (Development|PrintString "That's triggering!")
  (Utilities|Casting|CastToBP_MB_ProjectCharacter OtherActor)
  (Development|PrintString "Casting to player")
  (bind _output_get (Variables|Default|SetLevel%20Sequence (Variables|Default|GetLevel%20Sequence)))
  (if (Variables|Default|GetHasPlayed)
    (Development|PrintString "not more sequence for u >:(")
    (else
      (Development|PrintString "Sequence prepared")
      (bind _returnvalue (Sequencer|Player|CreateLevelSequencePlayer _output_get (Variables|Default|GetSequenceSettings)))
      (Sequencer|Player|Play _returnvalue :!class /Script/MovieScene.MovieSceneSequencePlayer)
      (Development|PrintString "Playing video")
      (Variables|Default|SetHasPlayed true)
      (Development|PrintString "Has played!"))))

(event EventTick
  (params (DeltaSeconds :type Float%20%28single-precision%29)))

(fn ConstructionScript)